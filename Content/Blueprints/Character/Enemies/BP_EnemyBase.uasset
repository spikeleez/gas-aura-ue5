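; BP_EnemyBase is the base enemy Blueprint, handling attack-facing updates and dissolve visuals for body and weapon.
; UpdateFacingTargetLocation writes the given location to the Motion Warping "FacingTarget" warp target so warped animations can orient toward it.
; Two events store the supplied dynamic material instances, then play separate timelines that drive each one's "Dissolve" scalar parameter.
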(event EventStartDissolveTimeline
  (params (DynamicMaterialInstance :type Material%20Instance%20Dynamic%20Object%20Reference))
  (Variables|Character|Materials|SetDynamicBodyDissolveMaterialInstance DynamicMaterialInstance)
  (bind _dissolvetrack (Timeline|DissolveTimeline Play)
    (:Update
      (Rendering|Material|SetScalarParameterValue (Variables|Character|Materials|GetDynamicBodyDissolveMaterialInstance) "Dissolve" _dissolvetrack :!class /Script/Engine.MaterialInstanceDynamic))))

(event EventStartWeaponDissolveTimeline
  (params (DynamicMaterialInstance :type Material%20Instance%20Dynamic%20Object%20Reference))
  (Variables|Character|Materials|SetDynamicWeaponDissolveMaterialInstance DynamicMaterialInstance)
  (bind _weapondissolvetrack (Timeline|WeaponDissolveTimeline Play)
    (:Update
      (Rendering|Material|SetScalarParameterValue (Variables|Character|Materials|GetDynamicWeaponDissolveMaterialInstance) "Dissolve" _weapondissolvetrack :!class /Script/Engine.MaterialInstanceDynamic))))

(event EventUpdateFacingTargetLocation
  (params (Location :type Vector%20%28by%20ref%29 :default "0, 0, 0"))
  (Class|MotionWarpingComponent|AddorUpdateWarpTargetfromLocation (Variables|Default|GetMotionWarping) "FacingTarget" Location))

(fn ConstructionScript)