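; Aura player controller Blueprint that adds a debug attribute menu for inspecting actors under the cursor.
; Middle mouse, while an actor is hovered, creates WBP_DebugAttributeMenu targeting the cursor hit actor, replacing any menu already on screen.
; Caps Lock removes the menu and clears its reference.
; Both inputs use debug key events, and the hover state and cursor hit are read from variables this graph never sets.
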(event Input|MouseEvents|DebugKeyMiddleMouseButton
  (params (Key :type Key%20Structure :default "None") (ActionValue :type Input%20Action%20Value%20Structure))
  ;[1 1 1] Debug - Attribute Menu Widget
  (:Pressed
    (Debug|AttributeMenuWidget|CreateDebugAttributeMenuWidget)))

(event Input|KeyboardEvents|DebugKeyCapsLock
  (params (Key :type Key%20Structure :default "None") (ActionValue :type Input%20Action%20Value%20Structure))
  ;[1 1 1] Debug - Attribute Menu Widget
  (:Pressed
    (Debug|AttributeMenuWidget|DestroyAnyDebugAttributeMenuWidget)))

(fn ConstructionScript)

(fn CreateDebugAttributeMenuWidget
  (if (Variables|Default|GetbCursorIsHoveredActor)
    (Variables|Debug|AttributeMenuWidget|GetDebugAttributeMenuWidget
      (:then
        (Widget|RemovefromParent (Variables|Debug|AttributeMenuWidget|GetDebugAttributeMenuWidget))
        (Variables|Debug|AttributeMenuWidget|SetDebugAttributeMenuWidget 0)
        (bind _returnvalue (UserInterface|CreateWidget "/Game/Blueprints/UI/Debug/WBP_DebugAttributeMenu.WBP_DebugAttributeMenu_C" 0 (.HitActor (Collision|BreakHitResult (Variables|Default|GetCursorHit)))))
        (bind _output_get (Variables|Debug|AttributeMenuWidget|SetDebugAttributeMenuWidget _returnvalue))
        (UserInterface|Viewport|AddtoViewport _output_get 0))
      (:else
        (bind _returnvalue_2 (UserInterface|CreateWidget "/Game/Blueprints/UI/Debug/WBP_DebugAttributeMenu.WBP_DebugAttributeMenu_C" 0 (.HitActor (Collision|BreakHitResult (Variables|Default|GetCursorHit)))))
        (bind _output_get_2 (Variables|Debug|AttributeMenuWidget|SetDebugAttributeMenuWidget _returnvalue_2))
        (UserInterface|Viewport|AddtoViewport _output_get_2 0)))))

(fn DestroyAnyDebugAttributeMenuWidget
  (bind _debugattributemenuwidget (Variables|Debug|AttributeMenuWidget|GetDebugAttributeMenuWidget)
    (:then
      (Widget|RemovefromParent _debugattributemenuwidget)
      (Variables|Debug|AttributeMenuWidget|SetDebugAttributeMenuWidget 0))
    (:else)))