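; GA_FireBolt is the Fire Bolt gameplay ability, currently wired only to test targeting under the mouse.
; On activation it runs the TargetDataUnderMouse task, draws a debug sphere at the returned hit location and ends.
; A disconnected chain holds the intended cast: play the cast montage, await its gameplay event, spawn the projectile, then end shortly after input release.
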(event Ability|EventActivateAbility
  (bind _data (|TargetDataUnderMouse)
    (:ValidData
      (Rendering|Debug|DrawDebugSphere (.Location (Collision|BreakHitResult (Ability|TargetData|GetHitResultfromTargetData _data))) 64.0 12 "(R=1.000000,G=1.000000,B=1.000000,A=1.000000)" 2e+01)
      (Ability|EndAbility))))

(event Ability|EventOnEndAbility
  (params (bWasCancelled :type Boolean)))