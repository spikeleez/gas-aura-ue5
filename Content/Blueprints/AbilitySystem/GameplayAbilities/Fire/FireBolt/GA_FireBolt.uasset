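; Fire Bolt gameplay ability that casts a projectile spell toward the point under the mouse.
; On activation, it reads the cursor hit location, turns the avatar toward it via an interface message, and plays the cast montage.
; A montage gameplay event triggers the projectile spawn at the stored location.
; The ability then waits for input release and a short delay before ending.
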(event Ability|EventActivateAbility
  (bind _data (|TargetDataUnderMouse)
    (:ValidData
      (bind _output_get (Variables|Default|SetProjectileTargetLocation (.Location (Collision|BreakHitResult (Ability|TargetData|GetHitResultfromTargetData _data)))))
      (Class|CombatInterface|UpdateFacingTargetLocation(Message) (Ability|GetAvatarActorfromActorInfo) _output_get)
      (|PlayMontageandWaitProxy "None" "/Game/Assets/Characters/Aura/Animations/Abilities/AM_Cast_FireBolt.AM_Cast_FireBolt" 1.0 "None" true 1.0 0.0 false
        (:then
          (Ability|Tasks|WaitGameplayEvent "(TagName=\"GameplayEvent.Montage.FireBolt\")" 0 true
            (:EventReceived
              (Class|AuraProjectileSpell|SpawnProjectileSpell (Variables|Default|GetProjectileTargetLocation))
              (Ability|Tasks|WaitInputRelease true
                (:OnRelease
                  (Ability|Tasks|WaitDelay 0.3
                    (:OnFinish
                      (Ability|EndAbility))))))))))))

(event Ability|EventOnEndAbility
  (params (bWasCancelled :type Boolean)))