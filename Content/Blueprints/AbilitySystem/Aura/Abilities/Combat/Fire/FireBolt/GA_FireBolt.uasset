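; Fire Bolt gameplay ability that fires a projectile spell at the point under the mouse.
; A target data task supplies the hit location, then the avatar turns to face it and plays the attack montage.
; A montage gameplay event spawns the projectile, timing the shot to the animation.
; The ability ends shortly after input release following the shot, or when the montage completes, is interrupted or is cancelled.
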(event Ability|EventActivateAbility
  (bind _data (|TargetDataUnderMouse)
    (:ValidData
      (bind _output_get (Variables|Projectile|SetProjectileTargetLocation (.Location (Collision|BreakHitResult (Ability|TargetData|GetHitResultfromTargetData _data)))))
      (Class|CombatInterface|UpdateFacingTargetLocation(Message) (Ability|GetAvatarActorfromActorInfo) _output_get)
      (|PlayMontageandWaitProxy "None" (Variables|Default|GetAttackMontage) 1.0 "None" true 1.0 0.0 false
        (:then
          (Ability|Tasks|WaitGameplayEvent (Variables|Default|GetAttackMontageTag) 0 true
            (:EventReceived
              (Class|AuraProjectileAbility|SpawnProjectileSpell (Variables|Projectile|GetProjectileTargetLocation))
              (Ability|Tasks|WaitInputRelease true
                (:OnRelease
                  (Ability|Tasks|WaitDelay 0.3
                    (:OnFinish
                      (Ability|EndAbility))))))))
        (:OnCompleted
          (Ability|EndAbility :!label _label))
        (:OnInterrupted
          (goto _label))
        (:OnCancelled
          (goto _label))))))

(event Ability|EventOnEndAbility
  (params (bWasCancelled :type Boolean)))