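; GA_RangedAttack is an enemy gameplay ability that performs a ranged attack by firing a projectile spell at the combat target.
; On activation it turns the avatar toward the target, then plays the attack montage and waits once for the montage's gameplay event tag.
; That event spawns the projectile aimed at the target's location, and the ability ends when the montage completes, is interrupted or is cancelled.
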(event Ability|EventActivateAbility
  (Class|AuraAttackAbility|UpdateAvatarFacingTarget)
  (Utilities|PlayAttackMontageandWaitGameplayEvent
    (:EventReceived
      (Class|AuraProjectileAbility|SpawnProjectileSpell (Class|AuraAttackAbility|GetCombatTargetLocation)))))

(event Ability|EventOnEndAbility
  (params (bWasCancelled :type Boolean)))