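; Gameplay ability for an enemy melee attack that damages a hostile player in range.
; On activation it turns the avatar toward its target, plays the attack montage and waits for a single gameplay event matching the montage tag.
; That event triggers damage on the first non-friendly live player found within the attack socket's radius.
; The ability ends when the montage completes, is interrupted or is cancelled.
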(event Ability|EventActivateAbility
  (Class|AuraAttackAbility|UpdateAvatarFacingTarget)
  (Utilities|PlayAttackMontageandWaitGameplayEvent
    (:EventReceived
      (Class|AuraDamageGameplayAbility|CauseDamage (MeleeAbility|Combat|GetCombatTargetinAttackRadius)))))

(event Ability|EventOnEndAbility
  (params (bWasCancelled :type Boolean)))

(fn GetCombatTargetinAttackRadius
  (bind _outoverlappingactors (Class|AuraAbilitySystemLibrary|GetLivePlayersWithinRadius self (Utilities|Array|MakeArray (Ability|GetAvatarActorfromActorInfo)) (Class|AuraAttackAbility|GetAttackSocketRadius) (Class|AuraAttackAbility|GetCombatSocketLocation)))
  (for _array_element _outoverlappingactors
    (bind _output_get (LocalVariables|SetCombatTarget _array_element))
    (if (Class|AuraAbilitySystemLibrary|IsNotFriend _output_get (Ability|GetAvatarActorfromActorInfo))
      (return (LocalVariables|GetCombatTarget)))))